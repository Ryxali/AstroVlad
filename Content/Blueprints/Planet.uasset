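; Planet actor that populates itself with victim pawns when play begins.
; BeginPlay calls SpawnVictim nine times, each spawning a VictimPawn at a random point on a fixed-radius sphere around the actor's location.
; Each pawn receives a reference to this planet on spawn; overlap and tick events are unused.
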(event `self.ReceiveBeginPlay`
  (`self.SpawnVictim`)
  (`self.SpawnVictim`)
  (`self.SpawnVictim`)
  (`self.SpawnVictim`)
  (`self.SpawnVictim`)
  (`self.SpawnVictim`)
  (`self.SpawnVictim`)
  (`self.SpawnVictim`)
  (`self.SpawnVictim`))

(event `self.ReceiveActorBeginOverlap`
  (params (OtherActor :type "Actor Object Reference")))

(event `self.ReceiveTick`
  (params (DeltaSeconds :type "Float (single-precision)")))

(fn `SpawnVictim`
  (`|SpawnActorFromClass` "/Game/Blueprints/VictimPawn.VictimPawn_C" (`KismetMathLibrary.Conv_VectorToTransform` (+ (`self.K2_GetActorLocation`) (* (`KismetMathLibrary.RandomUnitVector`) 5000))) "Undefined" "OverrideRootScale" null self))

(fn `UserConstructionScript`)