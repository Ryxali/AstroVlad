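; Victim pawn that lives on the surface of a Planet actor and relocates when killed.
; Construction finds and attaches to the Planet, then Align traces toward its center to snap the pawn to the surface normal, rejecting SpawnBlock-tagged components.
; Kill spawns a particle effect on the Planet, then retries random offsets through Align up to a fixed limit.
; GetSpeed returns zero; AlignPosition and AlignRotation are not called here.
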(event `self.ReceiveBeginPlay`)

(event `self.ReceiveActorBeginOverlap`
  (params (OtherActor :type "Actor Object Reference")))

(event `self.ReceiveTick`
  (params (DeltaSeconds :type "Float (single-precision)")))

(event `Kill`
  (bind _skeletalmesh (`self.SkeletalMesh`))
  (`GameplayStatics.SpawnEmitterAttached` "/Game/Particles/BloodAndThunder.BloodAndThunder" (`/Game/Blueprints/Planet.DefaultSceneRoot` (`self.Planet`)) "None" (`SceneComponent.K2_GetComponentLocation` _skeletalmesh) (`SceneComponent.K2_GetComponentRotation` _skeletalmesh) "KeepWorldPosition")
  (for _index (range 1 (+ 20 1))
    (bind _success (`self.SetRandomPosition`))
    (if _success
      (break)))
  (if (== _index 20)
    (`KismetSystemLibrary.PrintString` "NO FIND PLACE")))

(fn `Align`
  (returns (Success :type Boolean))
  (bind (_outhit _returnvalue) (`KismetSystemLibrary.LineTraceSingleForObjects` :`Start` (`self.K2_GetActorLocation`) :`End` (`self.K2_GetActorLocation` (`self.Planet`)) :`ObjectTypes` (`|MakeArray` "ObjectTypeQuery1" "ObjectTypeQuery2" :!type "EObjectTypeQuery Enum") :`DrawDebugType` "Persistent"))
  (if _returnvalue
    (bind (_bblockinghit _binitialoverlap _time _location _impactpoint _normal _impactnormal _physmat _hitactor _hitcomponent) (`GameplayStatics.BreakHitResult` _outhit))
    (if (`ActorComponent.ComponentHasTag` _hitcomponent "SpawnBlock")
      _
      (else
        (`self.K2_SetActorLocation` _impactpoint)
        (`self.SetActorRotation` (`KismetMathLibrary.MakeRotFromZ` _normal))
        (return true))))
  (return false))

(fn `AlignPosition`
  (returns (Success :type Boolean))
  (bind (_outhit _returnvalue) (`KismetSystemLibrary.LineTraceSingleForObjects` :`Start` (`self.K2_GetActorLocation`) :`End` (`self.K2_GetActorLocation` (`self.Planet`)) :`ObjectTypes` (`|MakeArray` "ObjectTypeQuery1" "ObjectTypeQuery2" :!type "EObjectTypeQuery Enum") :`bTraceComplex` true :`DrawDebugType` "Persistent"))
  (if _returnvalue
    (bind (_bblockinghit _binitialoverlap _time _location _impactpoint _normal _impactnormal _physmat _hitactor _hitcomponent) (`GameplayStatics.BreakHitResult` _outhit))
    (`self.K2_SetActorLocation` _location)
    (return (not (`ActorComponent.ComponentHasTag` _hitcomponent "SpawnBlock")))
    (else
      (`KismetSystemLibrary.PrintString` "Hello")
      (return false))))

(fn `AlignRotation`
  (bind _planet (`self.Planet`))
  (`/Engine/EditorBlueprintResources/StandardMacros.IsValid` (`self.Planet`)
    (:`Is Valid`
      _)
    (:`Is Not Valid`
      (bind _outactors (`GameplayStatics.GetAllActorsOfClass` "/Game/Blueprints/Planet.Planet_C"))
      (set `self.Planet` (`KismetArrayLibrary.Array_Get` _outactors))))
  (`self.K2_AttachRootComponentToActor` _planet "None" "KeepWorldPosition")
  (`self.SetActorRotation` (`KismetMathLibrary.MakeRotFromZ` (`KismetMathLibrary.Normal` (- (`self.K2_GetActorLocation`) (`self.K2_GetActorLocation` _planet))))))

(fn `GetSpeed`
  (returns (Speed :type "Float (double-precision)"))
  (return 0.0))

(fn `SetRandomPosition`
  (returns (Success :type Boolean))
  (`self.K2_SetActorLocation` (+ (`self.K2_GetActorLocation`) (* (`KismetMathLibrary.RandomUnitVector`) 5000)))
  (bind _success (`self.Align`))
  (return _success))

(fn `UserConstructionScript`
  (`/Engine/EditorBlueprintResources/StandardMacros.IsValid` (`self.Planet`)
    (:`Is Valid`
      _)
    (:`Is Not Valid`
      (bind _outactors (`GameplayStatics.GetAllActorsOfClass` "/Game/Blueprints/Planet.Planet_C"))
      (set `self.Planet` (`KismetArrayLibrary.Array_Get` _outactors))))
  (`self.K2_AttachRootComponentToActor` (`self.Planet`) "None" "KeepWorldPosition")
  (for _index (range 1 (+ 20 1))
    (bind _success (`self.Align`))
    (if _success
      (break)))
  (if (== _index 20)
    (`KismetSystemLibrary.PrintString` "NO FIND PLACE")))