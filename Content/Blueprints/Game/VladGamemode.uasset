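; Game mode that holds the game's highscore list and persists it through a VladSaveGame in the "Highscore" slot.
; The construction script loads the saved list, or fills it with identical placeholder entries when no valid save is found.
; AddHighscore only appends an entry, while SaveHighscores separately writes the list into a fresh save object.
; GetElapsedTime exposes the GameState's match-dependent elapsed time.
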(event `self.ReceiveBeginPlay`)

(event `self.ReceiveTick`
  (params (DeltaSeconds :type "Float (single-precision)")))

(fn `AddHighscore`
  (params (entry :type "/Game/Blueprints/Game/HighscoreEntry Structure"))
  (`KismetArrayLibrary.Array_Add` (`self.Highscores`) entry))

(fn `GetElapsedTime`
  (returns (time :type Integer))
  ;[1 1 1] This is dependant on GameState and "match". AGameState::ElapsedTime for more.
  (return (`GameState.ElapsedTime` (`GameplayStatics.GetGameState`))))

(fn `LoadHighscores`
  (bind _highscores (`self.Highscores`))
  (bind _returnvalue (`GameplayStatics.LoadGameFromSlot` "Highscore"))
  (bind _asvlad_save_game (cast `/Game/Blueprints/Game/VladSaveGame` _returnvalue)
    (:`then`
      (set `self.Highscores` (`/Game/Blueprints/Game/VladSaveGame.Highscores` _asvlad_save_game)))
    (:`CastFailed`
      ;[1 1 1] Default List
      (`KismetArrayLibrary.Array_Add` _highscores (make `/Game/Blueprints/Game/HighscoreEntry` "CRAIG HERNANDEZ"))
      (`KismetArrayLibrary.Array_Add` _highscores (make `/Game/Blueprints/Game/HighscoreEntry` "CRAIG HERNANDEZ"))
      (`KismetArrayLibrary.Array_Add` _highscores (make `/Game/Blueprints/Game/HighscoreEntry` "CRAIG HERNANDEZ"))
      (`KismetArrayLibrary.Array_Add` _highscores (make `/Game/Blueprints/Game/HighscoreEntry` "CRAIG HERNANDEZ"))
      (`KismetArrayLibrary.Array_Add` _highscores (make `/Game/Blueprints/Game/HighscoreEntry` "CRAIG HERNANDEZ"))
      (`KismetArrayLibrary.Array_Add` _highscores (make `/Game/Blueprints/Game/HighscoreEntry` "CRAIG HERNANDEZ")))))

(fn `SaveHighscores`
  (bind _returnvalue (`GameplayStatics.CreateSaveGameObject` "/Game/Blueprints/Game/VladSaveGame.VladSaveGame_C"))
  (bind _asvlad_save_game (cast `/Game/Blueprints/Game/VladSaveGame` _returnvalue))
  (for _array_element (`self.Highscores`)
    (`KismetArrayLibrary.Array_Add` (`/Game/Blueprints/Game/VladSaveGame.Highscores` _asvlad_save_game) _array_element))
  (`GameplayStatics.SaveGameToSlot` _returnvalue "Highscore"))

(fn `UserConstructionScript`
  (`self.LoadHighscores`))