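; VladHUD is a HUD Blueprint that shows the player's elapsed time and hunger on screen.
; On BeginPlay it casts the game mode to VladGameMode and resets that game mode's elapsed time.
; Each DrawHUD pass reads the formatted time and hunger value from the game mode and draws them as canvas text, with hunger truncated to an integer.
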(event `self.ReceiveBeginPlay`
  (bind _asvlad_game_mode (cast `/Game/Blueprints/Game/VladGamemode` (`GameplayStatics.GetGameMode`)))
  (`/Game/Blueprints/Game/VladGamemode.ResetElapsedTime` _asvlad_game_mode))

(event `self.ReceiveActorBeginOverlap`
  (params (OtherActor :type "Actor Object Reference")))

(event `self.ReceiveTick`
  (params (DeltaSeconds :type "Float (single-precision)")))

(event `self.ReceiveDrawHUD`
  (params (SizeX :type Integer) (SizeY :type Integer))
  (bind _asvlad_game_mode (cast `/Game/Blueprints/Game/VladGamemode` (`GameplayStatics.GetGameMode`)))
  (bind (_seconds _partial _formatedstring) (`/Game/Blueprints/Game/VladGamemode.GetElapsedTime` _asvlad_game_mode))
  (`self.DrawText` (`KismetStringLibrary.Concat_StrStr` "Elapsed Time: " _formatedstring) (struct :`R` 0.028124 :`G` 0.072072 :`B` 0.145 :`A` 1.0) 64.0 32.0 null 1.5)
  (bind _hunger (`/Game/Blueprints/Game/VladGamemode.GetHunger` _asvlad_game_mode))
  (`self.DrawText` (`KismetStringLibrary.Concat_StrStr` "Hunger: " (`KismetStringLibrary.Conv_IntToString` (`KismetMathLibrary.FTrunc` _hunger))) (struct :`A` 1) 64.0 64.0 null 1.5))

(fn `UserConstructionScript`)